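; Game mode for a local multiplayer bomber game that creates players, times the match and records death scores.
; BeginPlay gathers player and AI spawn points; SpawnPlayer swaps in characters with per-player materials on a shared camera.
; Player 1's spawn activates AI movement and a countdown Timeline that flags game over; the GameOver event pauses, then restarts the level.
; SaveGame accumulates both players' deaths in the Score slot, while LoadGame is an empty stub.
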(event `self.ReceiveTick`
  (params (DeltaSeconds :type "Float (single-precision)")))

(event `self.ReceiveBeginPlay`
  (bind _numberofplayers (`self.NumberOfPlayers`))
  (`|ExecutionSequence`
    (:`then_0`
      (while (<= _numberofplayers 2)
        (set `self.NumberOfPlayers` (+ _numberofplayers 1))
        (`GameplayStatics.CreatePlayer` -1)))
    (:`then_1`
      ;[1 1 1] Assign the array of player starts
      (bind _outactors (`GameplayStatics.GetAllActorsOfClass` "/Game/Blueprints/PlayerStartBomber.PlayerStartBomber_C"))
      (set `self.SpawnPoints` _outactors))
    (:`then_2`
      ;[1 1 1] Assign the array of spawn points
      (bind _outactors_2 (`GameplayStatics.GetAllActorsOfClass` "/Game/Blueprints/AiSpawnPoints.AiSpawnPoints_C"))
      (set `self.AISpawnPoints` _outactors_2))
    (:`then_3`
      ;[1 1 1] Create a save game
      (bind _returnvalue (`GameplayStatics.DoesSaveGameExist` "Score"))
      (if (not _returnvalue)
        (bind _returnvalue_2 (`GameplayStatics.CreateSaveGameObject` "/Game/Blueprints/SaveGameBomber.SaveGameBomber_C"))
        (bind _output_get (set `/Game/Blueprints/SaveGameBomber.SaveGameInstance` _returnvalue_2 _returnvalue_2))
        (`GameplayStatics.SaveGameToSlot` _output_get "Score")))))

(event `SpawnPlayer`
  (params (PlayerController :type "PlayerController Object Reference"))
  (bind _returnvalue (`Controller.K2_GetPawn` PlayerController))
  ;[1 1 1] Keep a track of player indices
  (set `self.PlayerIndex` (+ (`self.PlayerIndex`) 1))
  (`/Engine/EditorBlueprintResources/StandardMacros.IsValid` _returnvalue
    (:`Is Valid`
      (`self.K2_DestroyActor` _returnvalue)
      (bind _returnvalue_2 (`|SpawnActorFromClass` "/Game/Blueprints/PlayerCharacter.PlayerCharacter_C" (`self.SpawnTransform`) "Undefined" "OverrideRootScale" null null))
      (`Controller.Possess` PlayerController _returnvalue_2)
      (`PlayerController.SetViewTargetWithBlend` PlayerController (`self.GameCamera`) 0.0 "VTBlend_Linear" 0.0 false)
      (`/Engine/EditorBlueprintResources/StandardMacros.IsValid` (`self.Player1`)
        (:`Is Valid`
          ;[1 1 1] Appropriate player references
          (bind _output_get (set `self.Player2` _returnvalue_2))
          (`PrimitiveComponent.SetMaterial` (`Character.Mesh` _output_get) 0 "/Game/Mannequin/Character/Materials/M_UE4Man_BodyPlayer2.M_UE4Man_BodyPlayer2")
          (set `self.bPlayer2Dead` false))
        (:`Is Not Valid`
          (bind _output_get_2 (set `self.Player1` _returnvalue_2))
          (`PrimitiveComponent.SetMaterial` (`Character.Mesh` _output_get_2) 0 "/Game/Mannequin/Character/Materials/M_UE4Man_BodyPlayer1.M_UE4Man_BodyPlayer1")
          ;[1 1 1] Activate AI
          (bind _outactors (`GameplayStatics.GetAllActorsOfClass` "/Game/Blueprints/AICharacter.AICharacter_C"))
          (for _array_element _outactors
            (`ActorComponent.Activate` (`Character.CharacterMovement` _array_element) false)
            ;[1 1 1] Counts down the game time remaining
            (bind (_direction _gametimeremaining) (`Timeline|Timeline_0` :!via `PlayFromStart`)
              (:`Update`
                (set `self.Countdown` _gametimeremaining))
              (:`Finished`
                (set `self.bGameOver` true)))))))))

(event `GameOver`
  ;[1 1 1] Check if the game is over and reset
  (`GameplayStatics.SetGamePaused` true)
  (`KismetSystemLibrary.Delay` 5.0)
  (`self.RestartLevel`))

(event `RestartLevel`
  ;[1 1 1] Check if the game is over and reset
  (`GameplayStatics.SetGamePaused` false)
  (`KismetSystemLibrary.ExecuteConsoleCommand` "RestartLevel"))

(fn `LoadGame`
  (returns (Player1DeathScore :type Integer) (Player2DeathScore :type Integer)))

(fn `SaveGame`
  (params (Player1Death :type Integer) (Player2Death :type Integer))
  ;[1 1 1] SaveGame to slot
  (bind _returnvalue (`GameplayStatics.LoadGameFromSlot` "Score"))
  (`/Engine/EditorBlueprintResources/StandardMacros.IsValid` _returnvalue
    (:`Is Valid`
      (bind _assave_game_bomber (cast `/Game/Blueprints/SaveGameBomber` _returnvalue))
      (bind _output_get (set `/Game/Blueprints/SaveGameBomber.SaveGameInstance` _assave_game_bomber _assave_game_bomber))
      (set `/Game/Blueprints/SaveGameBomber.Player1DeathScore` (+ (`/Game/Blueprints/SaveGameBomber.Player1DeathScore` _output_get) Player1Death) _assave_game_bomber)
      (set `/Game/Blueprints/SaveGameBomber.Player2DeathScore` (+ (`/Game/Blueprints/SaveGameBomber.Player2DeathScore` _output_get) Player2Death) _assave_game_bomber)
      (bind _output_get_2 (set `/Game/Blueprints/SaveGameBomber.SaveSlotName` "Score" _assave_game_bomber))
      (`GameplayStatics.SaveGameToSlot` _output_get _output_get_2))
    (:`Is Not Valid`
      (bind _returnvalue_2 (`GameplayStatics.CreateSaveGameObject` "/Game/Blueprints/SaveGameBomber.SaveGameBomber_C"))
      (bind _output_get_3 (set `/Game/Blueprints/SaveGameBomber.SaveGameInstance` _returnvalue_2 _returnvalue_2))
      (if (`self.bPlayer1Dead`)
        (set `/Game/Blueprints/SaveGameBomber.Player1DeathScore` 1 _output_get_3))
      (if (`self.bPlayer2Dead`)
        (set `/Game/Blueprints/SaveGameBomber.Player2DeathScore` 1 _output_get_3))
      (bind _output_get_4 (set `/Game/Blueprints/SaveGameBomber.SaveSlotName` "Score" _output_get_3))
      (`GameplayStatics.SaveGameToSlot` _output_get_3 _output_get_4))))

(fn `UserConstructionScript`)