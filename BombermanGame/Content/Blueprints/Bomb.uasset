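; Bomberman-style bomb actor that explodes in a cross after a fuse, or on RemoteDetonate with a timed fallback.
; Prebuilt box collision and particle chains form the arms, trimmed without the longer-blast pickup and cut behind unbreakable walls on overlap.
; Detonation applies the explosion template, then DamageSurrounding kills players and AI and destroys pickups and breakable walls, which drop pickups.
; Deaths are reported to BomberGamemode before the bomb destroys itself.
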(event `RemoteDetonate`
  (bind _airef (`self.AIRef`))
  (bind _playerref (`self.PlayerRef`))
  (`/Engine/EditorBlueprintResources/StandardMacros.DoOnce` false :!label _label
    (:`Completed`
      ;[1 1 1] Switch remote detonate off
      (set `/Game/Blueprints/PlayerCharacter.RemoteDetonate` false (`self.PlayerRef`))
      ;[1 1 1] Spawn explosion
      (`self.IsParticleSystemValid` (`self.ParticleSystem9`) :!label _label_2)
      (`self.IsParticleSystemValid` (`self.ParticleSystem`))
      (`self.IsParticleSystemValid` (`self.ParticleSystem11`))
      (`self.IsParticleSystemValid` (`self.ParticleSystem2`))
      (`self.IsParticleSystemValid` (`self.ParticleSystem3`))
      (`self.IsParticleSystemValid` (`self.ParticleSystem4`))
      (`self.IsParticleSystemValid` (`self.ParticleSystem5`))
      (`self.IsParticleSystemValid` (`self.ParticleSystem6`))
      (`self.IsParticleSystemValid` (`self.ParticleSystem7`))
      (`self.IsParticleSystemValid` (`self.ParticleSystem8`))
      (`self.IsParticleSystemValid` (`self.ParticleSystem1`))
      (`self.IsParticleSystemValid` (`self.ParticleSystem12`))
      (`self.IsParticleSystemValid` (`self.ParticleSystem13`))
      (`self.IsParticleSystemValid` (`self.ParticleSystem14`))
      (`self.IsParticleSystemValid` (`self.ParticleSystem15`))
      (`self.IsParticleSystemValid` (`self.ParticleSystem16`))
      (`self.IsParticleSystemValid` (`self.ParticleSystem17`))
      (`self.IsParticleSystemValid` (`self.ParticleSystem18`))
      (`self.IsParticleSystemValid` (`self.ParticleSystem19`))
      (`self.IsParticleSystemValid` (`self.ParticleSystem20`))
      (`self.IsParticleSystemValid` (`self.ParticleSystem10`))
      ;[1 1 1] Setting bomb count
      (`/Engine/EditorBlueprintResources/StandardMacros.IsValid` _playerref
        (:`Is Valid`
          (set `/Game/Blueprints/PlayerCharacter.BombCount` 1 _playerref))
        (:`Is Not Valid`
          _))
      ;[1 1 1] Checking For breakable walls and players to cause damage
      (`|ExecutionSequence`
        (:`then_0`
          (`self.DamageSurrounding` (`self.BoxCollisionY`)))
        (:`then_1`
          (`self.DamageSurrounding` (`self.BoxCollisionX`)))
        (:`then_2`
          (`self.DamageSurrounding` (`self.BoxCollisionY2`)))
        (:`then_3`
          (`self.DamageSurrounding` (`self.BoxCollisionY3`)))
        (:`then_4`
          (`self.DamageSurrounding` (`self.BoxCollisionY4`)))
        (:`then_5`
          (`self.DamageSurrounding` (`self.BoxCollisionY5`)))
        (:`then_6`
          (`self.DamageSurrounding` (`self.BoxCollisionY6`)))
        (:`then_7`
          (`self.DamageSurrounding` (`self.BoxCollisionY7`)))
        (:`then_8`
          (`self.DamageSurrounding` (`self.BoxCollisionY8`)))
        (:`then_9`
          (`self.DamageSurrounding` (`self.BoxCollisionY9`)))
        (:`then_10`
          (`self.DamageSurrounding` (`self.BoxCollisionY10`)))
        (:`then_11`
          (`self.DamageSurrounding` (`self.BoxCollisionX2`)))
        (:`then_12`
          (`self.DamageSurrounding` (`self.BoxCollisionX3`)))
        (:`then_13`
          (`self.DamageSurrounding` (`self.BoxCollisionX4`)))
        (:`then_14`
          (`self.DamageSurrounding` (`self.BoxCollisionX5`)))
        (:`then_15`
          (`self.DamageSurrounding` (`self.BoxCollisionX6`)))
        (:`then_16`
          (`self.DamageSurrounding` (`self.BoxCollisionX7`)))
        (:`then_17`
          (`self.DamageSurrounding` (`self.BoxCollisionX8`)))
        (:`then_18`
          (`self.DamageSurrounding` (`self.BoxCollisionX9`)))
        (:`then_19`
          (`self.DamageSurrounding` (`self.BoxCollisionX10`))))
      (`KismetSystemLibrary.Delay` 1.5)
      (bind _asbomber_gamemode (cast `/Game/Blueprints/BomberGamemode` (`GameplayStatics.GetGameMode`)))
      (if (not (`/Game/Blueprints/BomberGamemode.bPlayer1Dead` _asbomber_gamemode))
        (set `/Game/Blueprints/BomberGamemode.bPlayer1Dead` (`self.IsPlayer1Dead`) _asbomber_gamemode))
      (if (not (`/Game/Blueprints/BomberGamemode.bPlayer2Dead` _asbomber_gamemode))
        (set `/Game/Blueprints/BomberGamemode.bPlayer2Dead` (`self.IsPlayer2Dead`) _asbomber_gamemode))
      (set `/Game/Blueprints/BomberGamemode.BothPlayersDead` (`self.BothPlayersDead?`) _asbomber_gamemode)
      (`/Engine/EditorBlueprintResources/StandardMacros.IsValid` _airef
        (:`Is Valid`
          (set `/Game/Blueprints/AICharacter.BombPlanted` false _airef))
        (:`Is Not Valid`
          _))
      (`self.K2_DestroyActor`))))

(event `self.ReceiveBeginPlay`
  (bind _playerref (`self.PlayerRef`))
  (`KismetSystemLibrary.Delay` 1.5)
  (`/Engine/EditorBlueprintResources/StandardMacros.IsValid` _playerref
    (:`Is Valid`
      (if (`/Game/Blueprints/PlayerCharacter.LongerBombBlastPickup` _playerref)
        (set `/Game/Blueprints/PlayerCharacter.LongerBombBlastPickup` false _playerref)
        (else
          ;[1 0.04167 0.04167] Longer Bomb blast. Fix it
          (`self.IsBoxCollisionValid` (`self.BoxCollisionY9`) :!label _label_3)
          (`self.IsBoxCollisionValid` (`self.BoxCollisionX4`))
          (`self.IsBoxCollisionValid` (`self.BoxCollisionX3`))
          (`self.IsBoxCollisionValid` (`self.BoxCollisionY8`))
          (`self.IsBoxCollisionValid` (`self.BoxCollisionY3`))
          (`self.IsBoxCollisionValid` (`self.BoxCollisionY10`))
          (`self.IsBoxCollisionValid` (`self.BoxCollisionX8`))
          (`self.IsBoxCollisionValid` (`self.BoxCollisionX9`))
          (`self.IsBoxCollisionValid` (`self.BoxCollisionX10`))
          (`self.IsBoxCollisionValid` (`self.BoxCollisionY5`))
          (`self.IsBoxCollisionValid` (`self.BoxCollisionY4`))
          (`self.IsBoxCollisionValid` (`self.BoxCollisionX5`))
          (`self.IsParticleSystemValidDestroy` (`self.ParticleSystem3`))
          (`self.IsParticleSystemValidDestroy` (`self.ParticleSystem4`))
          (`self.IsParticleSystemValidDestroy` (`self.ParticleSystem5`))
          (`self.IsParticleSystemValidDestroy` (`self.ParticleSystem8`))
          (`self.IsParticleSystemValidDestroy` (`self.ParticleSystem9`))
          (`self.IsParticleSystemValidDestroy` (`self.ParticleSystem10`))
          (`self.IsParticleSystemValidDestroy` (`self.ParticleSystem13`))
          (`self.IsParticleSystemValidDestroy` (`self.ParticleSystem14`))
          (`self.IsParticleSystemValidDestroy` (`self.ParticleSystem15`))
          (`self.IsParticleSystemValidDestroy` (`self.ParticleSystem18`))
          (`self.IsParticleSystemValidDestroy` (`self.ParticleSystem19`))
          (`self.IsParticleSystemValidDestroy` (`self.ParticleSystem20`)))))
    (:`Is Not Valid`
      (goto _label_3)))
  (`/Engine/EditorBlueprintResources/StandardMacros.IsValid` _playerref
    (:`Is Valid`
      (if (`/Game/Blueprints/PlayerCharacter.RemoteDetonate` _playerref)
        ;[1 1 1] Wait for 10 seconds and detonate automatically
        (`KismetSystemLibrary.Delay` 10.0)
        (goto _label)
        (else
          (goto _label_2))))
    (:`Is Not Valid`
      (goto _label_2))))

(event `self.BoxCollisionY.OnComponentBeginOverlap`
  (params (OverlappedComponent :type "PrimitiveComponent Object Reference") (OtherActor :type "Actor Object Reference") (OtherComp :type "PrimitiveComponent Object Reference") (OtherBodyIndex :type Integer) (bFromSweep :type Boolean) (SweepResult :type "HitResult Structure (by ref)"))
  ;[1 1 1] Deactivating particles based on unbreakable walls
  (bind _bunbreakablewallhit (`self.CheckOverLap` OtherActor (`self.ParticleSystem1`)))
  (if _bunbreakablewallhit
    (`self.IsParticleSystemValidHide` (`self.ParticleSystem3`))
    (`self.IsParticleSystemValidHide` (`self.ParticleSystem4`))
    (`self.IsParticleSystemValidHide` (`self.ParticleSystem5`))
    (`self.IsParticleSystemValidHide` (`self.ParticleSystem2`))
    (`self.IsBoxCollisionValid` (`self.BoxCollisionY4`))
    (`self.IsBoxCollisionValid` (`self.BoxCollisionY5`))
    (`self.IsBoxCollisionValid` (`self.BoxCollisionY2`))
    (`self.IsBoxCollisionValid` (`self.BoxCollisionY3`))))

(event `self.BoxCollisionX.OnComponentBeginOverlap`
  (params (OverlappedComponent :type "PrimitiveComponent Object Reference") (OtherActor :type "Actor Object Reference") (OtherComp :type "PrimitiveComponent Object Reference") (OtherBodyIndex :type Integer) (bFromSweep :type Boolean) (SweepResult :type "HitResult Structure (by ref)"))
  ;[1 1 1] Deactivating particles based on unbreakable walls
  (bind _bunbreakablewallhit (`self.CheckOverLap` OtherActor (`self.ParticleSystem11`)))
  (if _bunbreakablewallhit
    (`self.IsParticleSystemValidHide` (`self.ParticleSystem13`))
    (`self.IsParticleSystemValidHide` (`self.ParticleSystem14`))
    (`self.IsParticleSystemValidHide` (`self.ParticleSystem15`))
    (`self.IsParticleSystemValidHide` (`self.ParticleSystem12`))
    (`self.IsBoxCollisionValid` (`self.BoxCollisionX4`))
    (`self.IsBoxCollisionValid` (`self.BoxCollisionX5`))
    (`self.IsBoxCollisionValid` (`self.BoxCollisionX2`))
    (`self.IsBoxCollisionValid` (`self.BoxCollisionX3`))))

(event `self.BoxCollisionY2.OnComponentBeginOverlap`
  (params (OverlappedComponent :type "PrimitiveComponent Object Reference") (OtherActor :type "Actor Object Reference") (OtherComp :type "PrimitiveComponent Object Reference") (OtherBodyIndex :type Integer) (bFromSweep :type Boolean) (SweepResult :type "HitResult Structure (by ref)"))
  ;[1 1 1] Deactivating particles based on unbreakable walls
  (bind _bunbreakablewallhit (`self.CheckOverLap` OtherActor (`self.ParticleSystem2`)))
  (if _bunbreakablewallhit
    (`self.IsParticleSystemValidHide` (`self.ParticleSystem3`))
    (`self.IsParticleSystemValidHide` (`self.ParticleSystem4`))
    (`self.IsParticleSystemValidHide` (`self.ParticleSystem5`))
    (`self.IsBoxCollisionValid` (`self.BoxCollisionY4`))
    (`self.IsBoxCollisionValid` (`self.BoxCollisionY5`))
    (`self.IsBoxCollisionValid` (`self.BoxCollisionY3`))))

(event `self.BoxCollisionX2.OnComponentBeginOverlap`
  (params (OverlappedComponent :type "PrimitiveComponent Object Reference") (OtherActor :type "Actor Object Reference") (OtherComp :type "PrimitiveComponent Object Reference") (OtherBodyIndex :type Integer) (bFromSweep :type Boolean) (SweepResult :type "HitResult Structure (by ref)"))
  ;[1 1 1] Deactivating particles based on unbreakable walls
  (bind _bunbreakablewallhit (`self.CheckOverLap` OtherActor (`self.ParticleSystem12`)))
  (if _bunbreakablewallhit
    (`self.IsParticleSystemValidHide` (`self.ParticleSystem13`))
    (`self.IsParticleSystemValidHide` (`self.ParticleSystem14`))
    (`self.IsParticleSystemValidHide` (`self.ParticleSystem15`))
    (`self.IsBoxCollisionValid` (`self.BoxCollisionX4`))
    (`self.IsBoxCollisionValid` (`self.BoxCollisionX5`))
    (`self.IsBoxCollisionValid` (`self.BoxCollisionX3`))))

(event `self.BoxCollisionY3.OnComponentBeginOverlap`
  (params (OverlappedComponent :type "PrimitiveComponent Object Reference") (OtherActor :type "Actor Object Reference") (OtherComp :type "PrimitiveComponent Object Reference") (OtherBodyIndex :type Integer) (bFromSweep :type Boolean) (SweepResult :type "HitResult Structure (by ref)"))
  ;[1 1 1] Deactivating particles based on unbreakable walls
  (bind _bunbreakablewallhit (`self.CheckOverLap` OtherActor (`self.ParticleSystem3`)))
  (if _bunbreakablewallhit
    (`self.IsParticleSystemValidHide` (`self.ParticleSystem5`))
    (`self.IsParticleSystemValidHide` (`self.ParticleSystem2`))
    (`self.IsBoxCollisionValid` (`self.BoxCollisionY4`))
    (`self.IsBoxCollisionValid` (`self.BoxCollisionY5`))))

(event `self.BoxCollisionX3.OnComponentBeginOverlap`
  (params (OverlappedComponent :type "PrimitiveComponent Object Reference") (OtherActor :type "Actor Object Reference") (OtherComp :type "PrimitiveComponent Object Reference") (OtherBodyIndex :type Integer) (bFromSweep :type Boolean) (SweepResult :type "HitResult Structure (by ref)"))
  ;[1 1 1] Deactivating particles based on unbreakable walls
  (bind _bunbreakablewallhit (`self.CheckOverLap` OtherActor (`self.ParticleSystem13`)))
  (if _bunbreakablewallhit
    (`self.IsParticleSystemValidHide` (`self.ParticleSystem15`))
    (`self.IsParticleSystemValidHide` null)
    (`self.IsBoxCollisionValid` (`self.BoxCollisionX4`))
    (`self.IsBoxCollisionValid` (`self.BoxCollisionX5`))))

(event `self.BoxCollisionY4.OnComponentBeginOverlap`
  (params (OverlappedComponent :type "PrimitiveComponent Object Reference") (OtherActor :type "Actor Object Reference") (OtherComp :type "PrimitiveComponent Object Reference") (OtherBodyIndex :type Integer) (bFromSweep :type Boolean) (SweepResult :type "HitResult Structure (by ref)"))
  ;[1 1 1] Deactivating particles based on unbreakable walls
  (bind _bunbreakablewallhit (`self.CheckOverLap` OtherActor (`self.ParticleSystem4`)))
  (if _bunbreakablewallhit
    (`self.IsParticleSystemValidHide` (`self.ParticleSystem5`))
    (`self.IsBoxCollisionValid` (`self.BoxCollisionY5`))))

(event `self.BoxCollisionX4.OnComponentBeginOverlap`
  (params (OverlappedComponent :type "PrimitiveComponent Object Reference") (OtherActor :type "Actor Object Reference") (OtherComp :type "PrimitiveComponent Object Reference") (OtherBodyIndex :type Integer) (bFromSweep :type Boolean) (SweepResult :type "HitResult Structure (by ref)"))
  ;[1 1 1] Deactivating particles based on unbreakable walls
  (bind _bunbreakablewallhit (`self.CheckOverLap` OtherActor (`self.ParticleSystem14`)))
  (if _bunbreakablewallhit
    (`self.IsParticleSystemValidHide` (`self.ParticleSystem15`))
    (`self.IsBoxCollisionValid` (`self.BoxCollisionX5`))))

(event `self.BoxCollisionY5.OnComponentBeginOverlap`
  (params (OverlappedComponent :type "PrimitiveComponent Object Reference") (OtherActor :type "Actor Object Reference") (OtherComp :type "PrimitiveComponent Object Reference") (OtherBodyIndex :type Integer) (bFromSweep :type Boolean) (SweepResult :type "HitResult Structure (by ref)"))
  ;[1 1 1] Deactivating particles based on unbreakable walls
  (`self.CheckOverLap` OtherActor (`self.ParticleSystem5`)))

(event `self.BoxCollisionX5.OnComponentBeginOverlap`
  (params (OverlappedComponent :type "PrimitiveComponent Object Reference") (OtherActor :type "Actor Object Reference") (OtherComp :type "PrimitiveComponent Object Reference") (OtherBodyIndex :type Integer) (bFromSweep :type Boolean) (SweepResult :type "HitResult Structure (by ref)"))
  ;[1 1 1] Deactivating particles based on unbreakable walls
  (`self.CheckOverLap` OtherActor (`self.ParticleSystem15`)))

(event `self.BoxCollisionY6.OnComponentBeginOverlap`
  (params (OverlappedComponent :type "PrimitiveComponent Object Reference") (OtherActor :type "Actor Object Reference") (OtherComp :type "PrimitiveComponent Object Reference") (OtherBodyIndex :type Integer) (bFromSweep :type Boolean) (SweepResult :type "HitResult Structure (by ref)"))
  ;[1 1 1] Deactivating particles based on unbreakable walls
  (bind _bunbreakablewallhit (`self.CheckOverLap` OtherActor (`self.ParticleSystem6`)))
  (if _bunbreakablewallhit
    (`self.IsParticleSystemValidHide` (`self.ParticleSystem8`))
    (`self.IsParticleSystemValidHide` (`self.ParticleSystem9`))
    (`self.IsParticleSystemValidHide` (`self.ParticleSystem10`))
    (`self.IsParticleSystemValidHide` (`self.ParticleSystem7`))
    (`self.IsBoxCollisionValid` (`self.BoxCollisionY9`))
    (`self.IsBoxCollisionValid` (`self.BoxCollisionY7`))
    (`self.IsBoxCollisionValid` (`self.BoxCollisionY10`))
    (`self.IsBoxCollisionValid` (`self.BoxCollisionY8`))))

(event `self.BoxCollisionX6.OnComponentBeginOverlap`
  (params (OverlappedComponent :type "PrimitiveComponent Object Reference") (OtherActor :type "Actor Object Reference") (OtherComp :type "PrimitiveComponent Object Reference") (OtherBodyIndex :type Integer) (bFromSweep :type Boolean) (SweepResult :type "HitResult Structure (by ref)"))
  ;[1 1 1] Deactivating particles based on unbreakable walls
  (bind _bunbreakablewallhit (`self.CheckOverLap` OtherActor (`self.ParticleSystem16`)))
  (if _bunbreakablewallhit
    (`self.IsParticleSystemValidHide` (`self.ParticleSystem17`))
    (`self.IsParticleSystemValidHide` (`self.ParticleSystem19`))
    (`self.IsParticleSystemValidHide` (`self.ParticleSystem20`))
    (`self.IsParticleSystemValidHide` (`self.ParticleSystem18`))
    (`self.IsBoxCollisionValid` (`self.BoxCollisionX8`))
    (`self.IsBoxCollisionValid` (`self.BoxCollisionX9`))
    (`self.IsBoxCollisionValid` (`self.BoxCollisionX10`))
    (`self.IsBoxCollisionValid` (`self.BoxCollisionX7`))))

(event `self.BoxCollisionY7.OnComponentBeginOverlap`
  (params (OverlappedComponent :type "PrimitiveComponent Object Reference") (OtherActor :type "Actor Object Reference") (OtherComp :type "PrimitiveComponent Object Reference") (OtherBodyIndex :type Integer) (bFromSweep :type Boolean) (SweepResult :type "HitResult Structure (by ref)"))
  ;[1 1 1] Deactivating particles based on unbreakable walls
  (bind _bunbreakablewallhit (`self.CheckOverLap` OtherActor (`self.ParticleSystem7`)))
  (if _bunbreakablewallhit
    (`self.IsParticleSystemValidHide` (`self.ParticleSystem8`))
    (`self.IsParticleSystemValidHide` (`self.ParticleSystem9`))
    (`self.IsParticleSystemValidHide` (`self.ParticleSystem10`))
    (`self.IsBoxCollisionValid` (`self.BoxCollisionY9`))
    (`self.IsBoxCollisionValid` (`self.BoxCollisionY10`))
    (`self.IsBoxCollisionValid` (`self.BoxCollisionY8`))))

(event `self.BoxCollisionX7.OnComponentBeginOverlap`
  (params (OverlappedComponent :type "PrimitiveComponent Object Reference") (OtherActor :type "Actor Object Reference") (OtherComp :type "PrimitiveComponent Object Reference") (OtherBodyIndex :type Integer) (bFromSweep :type Boolean) (SweepResult :type "HitResult Structure (by ref)"))
  ;[1 1 1] Deactivating particles based on unbreakable walls
  (bind _bunbreakablewallhit (`self.CheckOverLap` OtherActor (`self.ParticleSystem17`)))
  (if _bunbreakablewallhit
    (`self.IsParticleSystemValidHide` (`self.ParticleSystem18`))
    (`self.IsParticleSystemValidHide` (`self.ParticleSystem19`))
    (`self.IsParticleSystemValidHide` (`self.ParticleSystem20`))
    (`self.IsBoxCollisionValid` (`self.BoxCollisionX8`))
    (`self.IsBoxCollisionValid` (`self.BoxCollisionX9`))
    (`self.IsBoxCollisionValid` (`self.BoxCollisionX10`))))

(event `self.BoxCollisionY8.OnComponentBeginOverlap`
  (params (OverlappedComponent :type "PrimitiveComponent Object Reference") (OtherActor :type "Actor Object Reference") (OtherComp :type "PrimitiveComponent Object Reference") (OtherBodyIndex :type Integer) (bFromSweep :type Boolean) (SweepResult :type "HitResult Structure (by ref)"))
  ;[1 1 1] Deactivating particles based on unbreakable walls
  (bind _bunbreakablewallhit (`self.CheckOverLap` OtherActor (`self.ParticleSystem8`)))
  (if _bunbreakablewallhit
    (`self.IsParticleSystemValidHide` (`self.ParticleSystem9`))
    (`self.IsParticleSystemValidHide` (`self.ParticleSystem10`))
    (`self.IsBoxCollisionValid` (`self.BoxCollisionY9`))
    (`self.IsBoxCollisionValid` (`self.BoxCollisionY10`))))

(event `self.BoxCollisionX8.OnComponentBeginOverlap`
  (params (OverlappedComponent :type "PrimitiveComponent Object Reference") (OtherActor :type "Actor Object Reference") (OtherComp :type "PrimitiveComponent Object Reference") (OtherBodyIndex :type Integer) (bFromSweep :type Boolean) (SweepResult :type "HitResult Structure (by ref)"))
  ;[1 1 1] Deactivating particles based on unbreakable walls
  (bind _bunbreakablewallhit (`self.CheckOverLap` OtherActor (`self.ParticleSystem18`)))
  (if _bunbreakablewallhit
    (`self.IsParticleSystemValidHide` (`self.ParticleSystem19`))
    (`self.IsParticleSystemValidHide` (`self.ParticleSystem20`))
    (`self.IsBoxCollisionValid` (`self.BoxCollisionX9`))
    (`self.IsBoxCollisionValid` (`self.BoxCollisionX10`))))

(event `self.BoxCollisionY9.OnComponentBeginOverlap`
  (params (OverlappedComponent :type "PrimitiveComponent Object Reference") (OtherActor :type "Actor Object Reference") (OtherComp :type "PrimitiveComponent Object Reference") (OtherBodyIndex :type Integer) (bFromSweep :type Boolean) (SweepResult :type "HitResult Structure (by ref)"))
  ;[1 1 1] Deactivating particles based on unbreakable walls
  (bind _bunbreakablewallhit (`self.CheckOverLap` OtherActor (`self.ParticleSystem9`)))
  (if _bunbreakablewallhit
    (`self.IsParticleSystemValidHide` (`self.ParticleSystem10`))
    (`self.IsBoxCollisionValid` (`self.BoxCollisionY10`))))

(event `self.BoxCollisionX9.OnComponentBeginOverlap`
  (params (OverlappedComponent :type "PrimitiveComponent Object Reference") (OtherActor :type "Actor Object Reference") (OtherComp :type "PrimitiveComponent Object Reference") (OtherBodyIndex :type Integer) (bFromSweep :type Boolean) (SweepResult :type "HitResult Structure (by ref)"))
  ;[1 1 1] Deactivating particles based on unbreakable walls
  (bind _bunbreakablewallhit (`self.CheckOverLap` OtherActor (`self.ParticleSystem19`)))
  (if _bunbreakablewallhit
    (`self.IsParticleSystemValidHide` (`self.ParticleSystem20`))
    (`self.IsBoxCollisionValid` (`self.BoxCollisionX10`))))

(event `self.BoxCollisionY10.OnComponentBeginOverlap`
  (params (OverlappedComponent :type "PrimitiveComponent Object Reference") (OtherActor :type "Actor Object Reference") (OtherComp :type "PrimitiveComponent Object Reference") (OtherBodyIndex :type Integer) (bFromSweep :type Boolean) (SweepResult :type "HitResult Structure (by ref)"))
  ;[1 1 1] Deactivating particles based on unbreakable walls
  (`self.CheckOverLap` null (`self.ParticleSystem10`)))

(event `self.BoxCollisionX10.OnComponentBeginOverlap`
  (params (OverlappedComponent :type "PrimitiveComponent Object Reference") (OtherActor :type "Actor Object Reference") (OtherComp :type "PrimitiveComponent Object Reference") (OtherBodyIndex :type Integer) (bFromSweep :type Boolean) (SweepResult :type "HitResult Structure (by ref)"))
  ;[1 1 1] Deactivating particles based on unbreakable walls
  (`self.CheckOverLap` OtherActor (`self.ParticleSystem20`)))

(fn `CheckOverLap`
  (params (OtherActor :type "Actor Object Reference") (ParticleSystem :type "ParticleSystemComponent Object Reference"))
  (returns (bUnbreakableWallHit :type Boolean) (bOverLapped :type Boolean))
  (bind _returnvalue (== (`GameplayStatics.GetObjectClass` OtherActor) "/Game/Blueprints/UnbreakableWalls.UnbreakableWalls_C"))
  (if _returnvalue
    (`SceneComponent.SetHiddenInGame` ParticleSystem true false)
    (`ActorComponent.Deactivate` ParticleSystem)
    (return _returnvalue false)))

(fn `DamageSurrounding`
  (params (CollisionBox :type "BoxComponent Object Reference"))
  (bind _sphere (`self.Sphere`))
  (`/Engine/EditorBlueprintResources/StandardMacros.IsValid` CollisionBox
    (:`Is Valid`
      ;[1 1 1] Checking for damage
      (for _array_element (`PrimitiveComponent.GetOverlappingActors` CollisionBox null)
        (bind _asbomber_gamemode (cast `/Game/Blueprints/BomberGamemode` (`GameplayStatics.GetGameMode`)))
        (bind _player1 (`/Game/Blueprints/BomberGamemode.Player1` _asbomber_gamemode))
        (if (== _array_element _player1)
          (`/Game/Blueprints/BomberGamemode.SaveGame` _asbomber_gamemode 1 0)
          (set `self.IsPlayer1Dead` true)
          (`/Engine/EditorBlueprintResources/StandardMacros.IsValid` _player1
            (:`Is Valid`
              (`self.PickupReset` _player1)
              (`self.SetActorHiddenInGame` _player1 true)
              (`PrimitiveComponent.SetCollisionEnabled` (`Character.CapsuleComponent` _player1) "NoCollision"))
            (:`Is Not Valid`
              _)))
        (bind _player2 (`/Game/Blueprints/BomberGamemode.Player2` _asbomber_gamemode))
        (if (== _array_element _player2)
          (`/Engine/EditorBlueprintResources/StandardMacros.IsValid` _player2
            (:`Is Valid`
              (`/Game/Blueprints/BomberGamemode.SaveGame` _asbomber_gamemode 0 1)
              (set `self.IsPlayer2Dead` true)
              (`self.PickupReset` _player2)
              (`self.SetActorHiddenInGame` _player2 true)
              (`PrimitiveComponent.SetCollisionEnabled` (`Character.CapsuleComponent` _player2) "NoCollision")
              (if (`self.IsPlayer1Dead`)
                (set `self.BothPlayersDead?` true))
              (if (== (`GameplayStatics.GetObjectClass` _array_element) "/Game/Blueprints/AICharacter.AICharacter_C") :!label _label
                (`self.K2_DestroyActor` _array_element)))
            (:`Is Not Valid`
              _))
          (else
            (goto _label)))
        (bind _returnvalue (`GameplayStatics.GetObjectClass` _array_element))
        ;;[1 1 1] Destroying Breakable wall
        (if (== _returnvalue "/Game/Blueprints/BreakableWall.BreakableWall_C")
          (bind _asbreakable_wall (cast `/Game/Blueprints/BreakableWall` _array_element))
          (`/Game/Blueprints/BreakableWall.DropPickup` _asbreakable_wall)
          (`self.K2_DestroyActor` _array_element)
          (else
            ;[1 1 1] Destroying Pickups
            (if (== _returnvalue "/Game/Blueprints/FasterRunSpeed.FasterRunSpeed_C")
              (`self.K2_DestroyActor` _array_element :!label _label_2)
              (elif (== _returnvalue "/Game/Blueprints/LongerBlast.LongerBlast_C")
                (goto _label_2)
                (elif (== _returnvalue "/Game/Blueprints/MoreBombs.MoreBombs_C")
                  (goto _label_2)
                  (elif (== _returnvalue "/Game/Blueprints/RemoteDetonate.RemoteDetonate_C")
                    (goto _label_2))))))))
      (`/Engine/EditorBlueprintResources/StandardMacros.IsValid` _sphere
        (:`Is Valid`
          (`ActorComponent.K2_DestroyComponent` _sphere))
        (:`Is Not Valid`
          _))
      (return))))

(fn `IsBoxCollisionValid`
  (params (BoxCollision :type "BoxComponent Object Reference"))
  (`/Engine/EditorBlueprintResources/StandardMacros.IsValid` BoxCollision
    (:`Is Valid`
      (`ActorComponent.K2_DestroyComponent` BoxCollision))
    (:`Is Not Valid`
      _))
  (return))

(fn `IsParticleSystemValid`
  (params (ParticleSystem :type "ParticleSystemComponent Object Reference"))
  (`/Engine/EditorBlueprintResources/StandardMacros.IsValid` ParticleSystem
    (:`Is Valid`
      (`ParticleSystemComponent.SetTemplate` ParticleSystem "/Game/StarterContent/Particles/P_Explosion.P_Explosion"))
    (:`Is Not Valid`
      _))
  (return))

(fn `IsParticleSystemValidDestroy`
  (params (ParticleSystem :type "ParticleSystemComponent Object Reference"))
  (`/Engine/EditorBlueprintResources/StandardMacros.IsValid` ParticleSystem
    (:`Is Valid`
      (`ActorComponent.K2_DestroyComponent` ParticleSystem))
    (:`Is Not Valid`
      _))
  (return))

(fn `IsParticleSystemValidHide`
  (params (ParticleSystem :type "ParticleSystemComponent Object Reference"))
  (`/Engine/EditorBlueprintResources/StandardMacros.IsValid` ParticleSystem
    (:`Is Valid`
      (`SceneComponent.SetHiddenInGame` ParticleSystem true false))
    (:`Is Not Valid`
      _))
  (return))

(fn `PickupReset`
  (params (PlayerRef :type "/Game/Blueprints/PlayerCharacter Object Reference"))
  (set `/Game/Blueprints/PlayerCharacter.BombCount` 0 PlayerRef)
  (set `/Game/Blueprints/PlayerCharacter.RunFasterPickup` false PlayerRef)
  (set `CharacterMovementComponent.MaxWalkSpeed` 600.0 (`Character.CharacterMovement` PlayerRef))
  (set `/Game/Blueprints/PlayerCharacter.LongerBombBlastPickup` false PlayerRef)
  (set `/Game/Blueprints/PlayerCharacter.RemoteDetonate` false PlayerRef))

(fn `UserConstructionScript`)