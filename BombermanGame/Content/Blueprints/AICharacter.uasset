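; AI character that roams among breakable and unbreakable walls and plants a bomb when the player comes within its sphere.
; Each Tick it moves forward and line-traces ahead, reversing at a Bomb.
; At either wall type, side traces for unbreakable walls make it prefer turning right, then left, then back.
; Sphere overlap spawns one Bomb, passes it a self reference and sets BombPlanted to block further drops.
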(event `self.ReceiveTick`
  (params (DeltaSeconds :type "Float (single-precision)"))
  (bind (_returnvalue_roll _returnvalue_pitch _returnvalue_yaw) (`KismetMathLibrary.BreakRotator` (`self.K2_GetActorRotation`)))
  (bind _cube (`self.Cube`))
  (bind _cuberight (`self.CubeRight`))
  (bind _cubeleft (`self.CubeLeft`))
  (bind (_returnvalue_roll_2 _returnvalue_pitch_2 _returnvalue_yaw_2) (`KismetMathLibrary.BreakRotator` (`self.K2_GetActorRotation` self)))
  (bind (_returnvalue_roll_3 _returnvalue_pitch_3 _returnvalue_yaw_3) (`KismetMathLibrary.BreakRotator` (`self.K2_GetActorRotation` self)))
  (bind _returnvalue (`SceneComponent.K2_GetComponentLocation` _cube))
  (bind _returnvalue_2 (`SceneComponent.K2_GetComponentLocation` _cuberight))
  (bind _returnvalue_3 (`SceneComponent.K2_GetComponentLocation` _cubeleft))
  (bind (_returnvalue_roll_4 _returnvalue_pitch_4 _returnvalue_yaw_4) (`KismetMathLibrary.BreakRotator` (`self.K2_GetActorRotation` self)))
  (bind (_returnvalue_roll_5 _returnvalue_pitch_5 _returnvalue_yaw_5) (`KismetMathLibrary.BreakRotator` (`self.K2_GetActorRotation` self)))
  (bind _returnvalue_4 (`KismetMathLibrary.GetForwardVector` (`SceneComponent.K2_GetComponentRotation` _cube)))
  ;[1 1 1] Move Forward
  (`self.AddMovementInput` _returnvalue_4 1.0 true)
  (bind _outhit (`KismetSystemLibrary.LineTraceSingle` _returnvalue (+ (* _returnvalue_4 95.0) _returnvalue) "TraceTypeQuery1"))
  (bind _returnvalue_5 (`GameplayStatics.GetObjectClass` (`.HitActor` (`GameplayStatics.BreakHitResult` _outhit))))
  (bind _returnvalue_6 (== _returnvalue_5 "/Game/Blueprints/BreakableWall.BreakableWall_C"))
  (if (or _returnvalue_6 (== _returnvalue_5 "/Game/Blueprints/UnbreakableWalls.UnbreakableWalls_C"))
    (bind _outhit_2 (`KismetSystemLibrary.LineTraceSingle` _returnvalue_2 (+ (* (`KismetMathLibrary.GetForwardVector` (`SceneComponent.K2_GetComponentRotation` _cuberight)) 75.0) _returnvalue_2) "TraceTypeQuery1"))
    (if (== (`GameplayStatics.GetObjectClass` (`.HitActor` (`GameplayStatics.BreakHitResult` _outhit_2))) "/Game/Blueprints/UnbreakableWalls.UnbreakableWalls_C")
      (bind _outhit_3 (`KismetSystemLibrary.LineTraceSingle` _returnvalue_3 (+ (* (`KismetMathLibrary.GetForwardVector` (`SceneComponent.K2_GetComponentRotation` _cubeleft)) 75.0) _returnvalue_3) "TraceTypeQuery1"))
      (if (== (`GameplayStatics.GetObjectClass` (`.HitActor` (`GameplayStatics.BreakHitResult` _outhit_3))) "/Game/Blueprints/UnbreakableWalls.UnbreakableWalls_C")
        (`self.K2_SetActorRotation` self (`KismetMathLibrary.MakeRotator` _returnvalue_roll_4 _returnvalue_pitch_4 (+ _returnvalue_yaw_4 180.0)) false)
        (else
          (`self.K2_SetActorRotation` self (`KismetMathLibrary.MakeRotator` _returnvalue_roll_2 _returnvalue_pitch_2 (+ _returnvalue_yaw_2 -90.0)) false)))
      (else
        (`self.K2_SetActorRotation` self (`KismetMathLibrary.MakeRotator` _returnvalue_roll_5 _returnvalue_pitch_5 (+ _returnvalue_yaw_5 90.0)) false)))
    (elif _returnvalue_6
      (if (`self.BombPlanted`)
        (`self.K2_SetActorRotation` (`KismetMathLibrary.MakeRotator` _returnvalue_roll _returnvalue_pitch (+ _returnvalue_yaw -90.0))))
      (elif (== _returnvalue_5 "/Game/Blueprints/Bomb.Bomb_C")
        (`self.K2_SetActorRotation` self (`KismetMathLibrary.MakeRotator` _returnvalue_roll_3 _returnvalue_pitch_3 (+ _returnvalue_yaw_3 180.0)) false)))))

(event `self.Sphere.OnComponentBeginOverlap`
  (params (OverlappedComponent :type "PrimitiveComponent Object Reference") (OtherActor :type "Actor Object Reference") (OtherComp :type "PrimitiveComponent Object Reference") (OtherBodyIndex :type Integer) (bFromSweep :type Boolean) (SweepResult :type "HitResult Structure (by ref)"))
  (if (== (`GameplayStatics.GetObjectClass` OtherActor) "/Game/Blueprints/PlayerCharacter.PlayerCharacter_C")
    (if (not (`self.BombPlanted`))
      (bind _returnvalue (`|SpawnActorFromClass` "/Game/Blueprints/Bomb.Bomb_C" (`self.MeshTransform`) "Undefined" "OverrideRootScale" null null))
      (set `/Game/Blueprints/Bomb.AIRef` self _returnvalue)
      (set `self.BombPlanted` true))))

(fn `UserConstructionScript`)