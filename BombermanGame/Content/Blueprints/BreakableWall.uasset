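; Breakable wall actor for what appears to be a Bomberman-style game, able to leave a power-up behind.
; DropPickup rolls roughly a 30% chance, then spawns one of four equally likely bomb or speed pickups at the Cube component's world location.
; The event graph and construction script are empty, so nothing in this Blueprint calls DropPickup or handles the wall breaking.
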(fn `DropPickup`
  (bind _returnvalue (`KismetMathLibrary.Conv_VectorToTransform` (`SceneComponent.K2_GetComponentLocation` (`self.Cube`))))
  (if (<= (`KismetMathLibrary.RandomIntegerInRange` 0 100) 30)
    (switch `int` (`KismetMathLibrary.RandomInteger` 4)
      (:`0`
        (`|SpawnActorFromClass` "/Game/Blueprints/MoreBombs.MoreBombs_C" _returnvalue "Undefined" "OverrideRootScale" null null))
      (:`1`
        (`|SpawnActorFromClass` "/Game/Blueprints/RemoteDetonate.RemoteDetonate_C" _returnvalue "Undefined" "OverrideRootScale" null null))
      (:`2`
        (`|SpawnActorFromClass` "/Game/Blueprints/FasterRunSpeed.FasterRunSpeed_C" _returnvalue "Undefined" "OverrideRootScale" null null))
      (:`3`
        (`|SpawnActorFromClass` "/Game/Blueprints/LongerBlast.LongerBlast_C" _returnvalue "Undefined" "OverrideRootScale" null null)))))

(fn `UserConstructionScript`)