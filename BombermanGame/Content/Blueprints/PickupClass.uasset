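; PickupClass is a pickup Actor that identifies which player overlaps it, with an empty event graph and construction script.
; DetectPlayerOnOverlap casts the actor to PlayerCharacter, skips it if PickedUp is set, then matches it to Player1 or Player2 in BomberGamemode.
; It returns that player and their UI control, which it first writes into the game mode's shared UIPlayerControl variable.
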(fn `DetectPlayerOnOverlap`
  (params (OtherActor :type "Actor Object Reference"))
  (returns (PlayerRef :type "/Game/Blueprints/PlayerCharacter Object Reference") (UIPlayerCOntrolRef :type "TextBlock Object Reference"))
  (bind _asplayer_character (cast `/Game/Blueprints/PlayerCharacter` OtherActor))
  (if (not (`/Game/Blueprints/PlayerCharacter.PickedUp` _asplayer_character))
    (bind _asbomber_gamemode (cast `/Game/Blueprints/BomberGamemode` (`GameplayStatics.GetGameMode`)))
    (bind _player1 (`/Game/Blueprints/BomberGamemode.Player1` _asbomber_gamemode))
    (if (== _player1 OtherActor)
      (set `self.PickupPlayerRef` _player1)
      (bind _asbomber_gamemode_2 (cast `/Game/Blueprints/BomberGamemode` (`GameplayStatics.GetGameMode`)))
      (set `/Game/Blueprints/BomberGamemode.UIPlayerControl` (`/Game/Blueprints/UIScreen.Player1Control` (`/Game/Blueprints/BomberGamemode.UIScreen` _asbomber_gamemode_2)) _asbomber_gamemode_2)
      (bind _asbomber_gamemode_3 (cast `/Game/Blueprints/BomberGamemode` (`GameplayStatics.GetGameMode`) :!label _label))
      (return (`self.PickupPlayerRef`) (`/Game/Blueprints/BomberGamemode.UIPlayerControl` _asbomber_gamemode_3))
      (else
        (bind _player2 (`/Game/Blueprints/BomberGamemode.Player2` _asbomber_gamemode))
        (if (== _player2 OtherActor)
          (set `self.PickupPlayerRef` _player2)
          (bind _asbomber_gamemode_4 (cast `/Game/Blueprints/BomberGamemode` (`GameplayStatics.GetGameMode`)))
          (set `/Game/Blueprints/BomberGamemode.UIPlayerControl` (`/Game/Blueprints/UIScreen.Player2Control` (`/Game/Blueprints/BomberGamemode.UIScreen` _asbomber_gamemode_4)) _asbomber_gamemode_4)
          (goto _label))))))

(fn `UserConstructionScript`)