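; HUD for a two-player Bomberman-style game that registers itself with BomberGamemode and creates the UIScreen widget on BeginPlay.
; The older canvas drawing of controls, countdown, round results and saved death scores is disconnected from DrawHUD, so it never runs.
; BlocksDestroyed sets BreakableWallsDone if any UnbreakableWalls actor is invalid, but nothing in this graph calls it.
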(event `self.ReceiveBeginPlay`
  (bind _asbomber_gamemode (cast `/Game/Blueprints/BomberGamemode` (`GameplayStatics.GetGameMode`)))
  (set `/Game/Blueprints/BomberGamemode.HudRef` self _asbomber_gamemode)
  ;[1 1 1] Adding this to the screen
  (bind _returnvalue (`|CreateWidget` "/Game/Blueprints/UIScreen.UIScreen_C" (`GameplayStatics.GetPlayerController` 0)))
  (`UserWidget.AddToViewport` _returnvalue 0)
  (bind _asbomber_gamemode_2 (cast `/Game/Blueprints/BomberGamemode` (`GameplayStatics.GetGameMode`)))
  (set `/Game/Blueprints/BomberGamemode.UIScreen` _returnvalue _asbomber_gamemode_2))

(event `self.ReceiveDrawHUD`
  (params (SizeX :type Integer) (SizeY :type Integer)))

(fn `BlocksDestroyed`
  (bind _outactors (`GameplayStatics.GetAllActorsOfClass` "/Game/Blueprints/UnbreakableWalls.UnbreakableWalls_C"))
  (for _array_element _outactors
    (`/Engine/EditorBlueprintResources/StandardMacros.IsValid` _array_element
      (:`Is Not Valid`
        (set `self.BreakableWallsDone` true)))))

(fn `Instructions`
  ;[1 1 1] Instructions
  (`self.DrawText` "Space / Start to start game" (struct :`A` 1.0) 1400.0 0.0 null 1.5)
  (`self.DrawText` "Green pickup : More Bombs" (struct :`A` 1.0) 1400.0 20.0 null 1.5)
  (`self.DrawText` "Blue pickup : Faster Run Speed" (struct :`A` 1.0) 1400.0 40.0 null 1.5)
  (`self.DrawText` "Orange pickup : Remote Bomb" (struct :`A` 1.0) 1400.0 60.0 null 1.5)
  (`self.DrawText` "Pink pickup :Longer Blasts" (struct :`A` 1.0) 1400.0 80.0 null 1.5)
  (`self.DrawText` "G or Gamepad button bottom for remote detonation" (struct :`A` 1.0) 1400.0 100.0 null 1.5)
  (`self.DrawText` "A/W/S/D and Left Stick for movements" (struct :`A` 1.0) 1400.0 120.0 null 1.5)
  (`self.DrawText` "F or Gamepad Button Down for placing bombs" (struct :`A` 1.0) 1400.0 140.0 null 1.5)
  (`self.DrawText` "R or Select on gamepad for Game Reset" (struct :`A` 1.0) 1400.0 160.0 null 1.5))

(fn `UserConstructionScript`)