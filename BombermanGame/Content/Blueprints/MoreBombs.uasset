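; MoreBombs is a pickup actor that sets the overlapping player's bomb count to a fixed value.
; It enables overlap events on its Cube and Box components after a short delay from BeginPlay.
; On Box overlap, DetectPlayerOnOverlap supplies player and UI references; for a valid player it flags the pickup, sets the count, shows a pickup message and destroys itself.
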(event `self.ReceiveBeginPlay`
  (`parent.ReceiveBeginPlay`)
  (`KismetSystemLibrary.Delay` 0.5)
  (set `PrimitiveComponent.bGenerateOverlapEvents` true (`self.Cube`))
  (set `PrimitiveComponent.bGenerateOverlapEvents` true (`self.Box`)))

(event `self.Box.OnComponentBeginOverlap`
  (params (OverlappedComponent :type "PrimitiveComponent Object Reference") (OtherActor :type "Actor Object Reference") (OtherComp :type "PrimitiveComponent Object Reference") (OtherBodyIndex :type Integer) (bFromSweep :type Boolean) (SweepResult :type "HitResult Structure (by ref)"))
  (bind (_playerref _uiplayercontrolref) (`self.DetectPlayerOnOverlap` OtherActor))
  (`/Engine/EditorBlueprintResources/StandardMacros.IsValid` _playerref
    (:`Is Valid`
      (set `/Game/Blueprints/PlayerCharacter.PickedUp` true _playerref)
      (set `/Game/Blueprints/PlayerCharacter.BombCount` 5 _playerref)
      (`TextBlock.SetText` _uiplayercontrolref "More Bombs Pickup")
      (`self.K2_DestroyActor`))))

(fn `UserConstructionScript`
  (`parent.UserConstructionScript`))